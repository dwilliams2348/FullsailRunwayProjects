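; BP_Modifier_Coin is a coin pickup that gives the player character a random temporary effect.
; When something overlaps its CoinPickup component, it casts to BP_ThirdPersonCharacter and ignores other actors.
; It then calls the character's ApplyEffect with one of four randomly selected enum effects and a random duration between MinEffectTime and MaxEffectTime, and runs OnPickup.
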(event `self.CoinPickup.OnComponentBeginOverlap`
  (params (OverlappedComponent :type "PrimitiveComponent Object Reference") (OtherActor :type "Actor Object Reference") (OtherComp :type "PrimitiveComponent Object Reference") (OtherBodyIndex :type Integer) (bFromSweep :type Boolean) (SweepResult :type "HitResult Structure (by ref)"))
  (bind _asbp_third_person_character (cast `/Game/GenericGame/Blueprints/Characters/BP_ThirdPersonCharacter` OtherActor))
  (`/Game/GenericGame/Blueprints/Characters/BP_ThirdPersonCharacter.ApplyEffect` _asbp_third_person_character (select `int` (`KismetMathLibrary.RandomIntegerInRange` 0 3) :`0` "NewEnumerator0" :`1` "NewEnumerator1" :`2` "NewEnumerator2" :`3` "NewEnumerator3" :!type "/Game/GenericGame/Blueprints/Enums/EEffects Enum") (`KismetMathLibrary.RandomFloatInRange` (`self.MinEffectTime`) (`self.MaxEffectTime`)))
  (`self.OnPickup`))

(fn `UserConstructionScript`
  (`parent.UserConstructionScript`))