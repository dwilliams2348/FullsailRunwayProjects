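; Parent Blueprint for coin pickups that add one to the third-person character's coin count on overlap.
; The CoinPickup component's overlap casts to BP_ThirdPersonCharacter, updates the count, then triggers OnPickup.
; If ShouldRespawn is set, OnPickup disables collision, hides the mesh and starts a one-shot RespawnTime timer to restore both.
; Otherwise, the coin destroys itself.
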(event `self.CoinPickup.OnComponentBeginOverlap`
  (params (OverlappedComponent :type "PrimitiveComponent Object Reference") (OtherActor :type "Actor Object Reference") (OtherComp :type "PrimitiveComponent Object Reference") (OtherBodyIndex :type Integer) (bFromSweep :type Boolean) (SweepResult :type "HitResult Structure (by ref)"))
  (bind _asbp_third_person_character (cast `/Game/GenericGame/Blueprints/Characters/BP_ThirdPersonCharacter` OtherActor))
  (`/Game/GenericGame/Blueprints/Characters/BP_ThirdPersonCharacter.UpdateCoinCount` _asbp_third_person_character 1)
  (`self.OnPickup`))

(event `RespawnCoin`
  (`PrimitiveComponent.SetCollisionEnabled` (`self.CoinPickup`) "QueryAndPhysics")
  (`SceneComponent.SetVisibility` (`self.StaticMesh`) true false))

(event `OnPickup`
  (if (`self.bShouldRespawn`)
    (`PrimitiveComponent.SetCollisionEnabled` (`self.CoinPickup`) "NoCollision")
    (`SceneComponent.SetVisibility` (`self.StaticMesh`) false false)
    (`KismetSystemLibrary.K2_SetTimerDelegate` (delegate `RespawnCoin`) (`self.RespawnTime`))
    (else
      (`self.K2_DestroyActor`))))

(fn `UserConstructionScript`)