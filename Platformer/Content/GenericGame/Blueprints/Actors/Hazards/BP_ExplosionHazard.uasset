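; Explosion hazard actor that fires a radial impulse and Niagara effect when the third-person character overlaps its SphereHit trigger.
; Impulse strength is randomized between min and max power once at BeginPlay.
; Each blast hides the Sphere component and disables its collision until a recharge timer restores both.
; SphereHit's own collision is left unchanged, and no flag gates overlaps during the recharge.
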(event `self.ReceiveBeginPlay`
  (set `RadialForceComponent.ImpulseStrength` (`KismetMathLibrary.RandomFloatInRange` (`self.MinExplosionPower`) (`self.MaxExplosionPower`)) (`self.RadialForce`)))

(event `self.SphereHit.OnComponentBeginOverlap`
  (params (OverlappedComponent :type "PrimitiveComponent Object Reference") (OtherActor :type "Actor Object Reference") (OtherComp :type "PrimitiveComponent Object Reference") (OtherBodyIndex :type Integer) (bFromSweep :type Boolean) (SweepResult :type "HitResult Structure (by ref)"))
  (bind _sphere (`self.Sphere`))
  (cast `/Game/GenericGame/Blueprints/Characters/BP_ThirdPersonCharacter` OtherActor)
  (`RadialForceComponent.FireImpulse` (`self.RadialForce`))
  (`NiagaraFunctionLibrary.SpawnSystemAtLocation` "/Game/ExternalAssets/ExplosionParticle/NS_Explosion.NS_Explosion" (`self.K2_GetActorLocation`))
  (`SceneComponent.SetVisibility` _sphere false false)
  (`PrimitiveComponent.SetCollisionEnabled` _sphere "NoCollision")
  (`KismetSystemLibrary.K2_SetTimerDelegate` (delegate `RenableExplosive`) (`self.RechargeTime`)))

(event `RenableExplosive`
  (bind _sphere (`self.Sphere`))
  (`SceneComponent.SetVisibility` _sphere true false)
  (`PrimitiveComponent.SetCollisionEnabled` _sphere "QueryAndPhysics"))

(fn `UserConstructionScript`)