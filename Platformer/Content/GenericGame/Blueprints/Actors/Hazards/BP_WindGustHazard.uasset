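; BP_WindGustHazard is a hazard actor that pushes the third-person player character with a constant wind force.
; On BeginPlay it rolls one horizontal force, with a direction limited to the positive X/Y quadrant and strength between MinWindForce and MaxWindForce.
; Bounds overlap events store or clear a single character reference, and Tick applies the force through that character's movement component while the reference is valid.
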(event `self.ReceiveBeginPlay`
  (set `self.ForceVector` (* (`KismetMathLibrary.Normal` (`KismetMathLibrary.MakeVector` (`KismetMathLibrary.RandomFloat`) (`KismetMathLibrary.RandomFloat`))) (`KismetMathLibrary.RandomFloatInRange` (`self.MinWindForce`) (`self.MaxWindForce`)))))

(event `self.ReceiveTick`
  (params (DeltaSeconds :type "Float (single-precision)"))
  (bind _characterref (`self.CharacterRef`)
    (:`then`
      (`CharacterMovementComponent.AddForce` (`Character.CharacterMovement` _characterref) (`self.ForceVector`)))
    (:`else`)))

(event `self.Bounds.OnComponentBeginOverlap`
  (params (OverlappedComponent :type "PrimitiveComponent Object Reference") (OtherActor :type "Actor Object Reference") (OtherComp :type "PrimitiveComponent Object Reference") (OtherBodyIndex :type Integer) (bFromSweep :type Boolean) (SweepResult :type "HitResult Structure (by ref)"))
  (bind _asbp_third_person_character (cast `/Game/GenericGame/Blueprints/Characters/BP_ThirdPersonCharacter` OtherActor))
  (set `self.CharacterRef` _asbp_third_person_character))

(event `self.Bounds.OnComponentEndOverlap`
  (params (OverlappedComponent :type "PrimitiveComponent Object Reference") (OtherActor :type "Actor Object Reference") (OtherComp :type "PrimitiveComponent Object Reference") (OtherBodyIndex :type Integer))
  (cast `/Game/GenericGame/Blueprints/Characters/BP_ThirdPersonCharacter` OtherActor)
  (set `self.CharacterRef` null))

(fn `UserConstructionScript`)