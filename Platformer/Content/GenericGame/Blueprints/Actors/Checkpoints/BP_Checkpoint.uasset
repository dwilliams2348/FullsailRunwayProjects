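; BP_Checkpoint is a checkpoint actor that registers itself as the third-person character's latest checkpoint when touched.
; It creates its "checkpoint reached" widget once at BeginPlay.
; Overlapping the Bounds component calls SetCheckpoint on the character, skipping repeats if this checkpoint is already its LastCheckpoint.
; A new activation also shows the widget, and a one-shot timer removes it after TextOnScreenTime.
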(event `self.ReceiveBeginPlay`
  (bind _returnvalue (`|CreateWidget` "/Game/GenericGame/Blueprints/Widgets/WBP_CheckpointReached.WBP_CheckpointReached_C"))
  (set `self.CheckpointHitText` _returnvalue))

(event `self.Bounds.OnComponentBeginOverlap`
  (params (OverlappedComponent :type "PrimitiveComponent Object Reference") (OtherActor :type "Actor Object Reference") (OtherComp :type "PrimitiveComponent Object Reference") (OtherBodyIndex :type Integer) (bFromSweep :type Boolean) (SweepResult :type "HitResult Structure (by ref)"))
  (bind _asbp_third_person_character (cast `/Game/GenericGame/Blueprints/Characters/BP_ThirdPersonCharacter` OtherActor))
  (if (not (== (`/Game/GenericGame/Blueprints/Characters/BP_ThirdPersonCharacter.LastCheckpoint` _asbp_third_person_character) self))
    (`/Game/GenericGame/Blueprints/Characters/BP_ThirdPersonCharacter.SetCheckpoint` _asbp_third_person_character self)
    (`UserWidget.AddToViewport` (`self.CheckpointHitText`) 0)
    (`KismetSystemLibrary.K2_SetTimerDelegate` (delegate `RemoveWidget`) (`self.TextOnScreenTime`))))

(event `RemoveWidget`
  (`Widget.RemoveFromParent` (`self.CheckpointHitText`)))

(fn `UserConstructionScript`)