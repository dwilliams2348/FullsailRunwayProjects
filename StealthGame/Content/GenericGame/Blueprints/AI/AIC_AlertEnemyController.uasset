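; AI controller for the alert enemy, which calls nearby patrol enemies to the player's location when it spots them.
; It runs the alert behavior tree, configures PawnSensing from the pawn's sight and hearing properties, and writes seen player and heard noise location to the Blackboard.
; A DoOnce gates the sphere-trace alert.
; A retriggerable delay detects lost sight, then clears the target, stops all patrol enemies' alerts and re-arms it.
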(event `self.ReceiveBeginPlay`
  (bind _pawnsensing (`self.PawnSensing`))
  ;[1 1 1] documented
  (`self.RunBehaviorTree` "/Game/GenericGame/Blueprints/AI/BT_AlertEnemy.BT_AlertEnemy")
  (bind _asbp_alert_enemy (cast `/Game/GenericGame/Blueprints/Characters/BP_AlertEnemy` (`self.K2_GetPawn`)))
  (`PawnSensingComponent.SetPeripheralVisionAngle` _pawnsensing (`/Game/GenericGame/Blueprints/Characters/BP_AlertEnemy.SightAngle` _asbp_alert_enemy))
  (set `PawnSensingComponent.SightRadius` (`/Game/GenericGame/Blueprints/Characters/BP_AlertEnemy.SightRadius` _asbp_alert_enemy) _pawnsensing)
  (bind _hearingrange (`/Game/GenericGame/Blueprints/Characters/BP_AlertEnemy.HearingRange` _asbp_alert_enemy))
  (set `PawnSensingComponent.HearingThreshold` _hearingrange _pawnsensing)
  (set `PawnSensingComponent.LOSHearingThreshold` (* _hearingrange 2.0) _pawnsensing))

(event `self.PawnSensing.OnSeePawn`
  (params (Pawn :type "Pawn Object Reference"))
  (bind _returnvalue (`self.K2_GetPawn`))
  (bind _ascharacter (cast `Character` Pawn :!pure true))
  (bind _returnvalue_2 (`self.K2_GetActorLocation` _returnvalue))
  ;[1 1 1] documented
  (if (== _ascharacter (`GameplayStatics.GetPlayerCharacter` 0))
    (`|ExecutionSequence`
      (:`then_0`
        (`/Engine/EditorBlueprintResources/StandardMacros.DoOnce` false :!label _label
          (:`Completed`
            (`BlackboardComponent.SetValueAsObject` (`self.Blackboard`) "TargetActor" _ascharacter)
            (bind _outhits (`KismetSystemLibrary.SphereTraceMultiForObjects` _returnvalue_2 _returnvalue_2 (`/Game/GenericGame/Blueprints/Characters/BP_AlertEnemy.AlertRadius` (cast `/Game/GenericGame/Blueprints/Characters/BP_AlertEnemy` _returnvalue :!pure true)) (`|MakeArray` "ObjectTypeQuery3" :!type "EObjectTypeQuery Enum") false (`|MakeArray` _returnvalue (`GameplayStatics.GetPlayerPawn` 0) :!type "Actor Object Reference")))
            (for _array_element _outhits
              (bind _asbp_patrol_enemy (cast `/Game/GenericGame/Blueprints/Characters/BP_PatrolEnemy` (`.HitActor` (`GameplayStatics.BreakHitResult` _array_element))))
              (`/Game/GenericGame/Blueprints/AI/AIC_PatrolEnemyController.OnStartAlert` (cast `/Game/GenericGame/Blueprints/AI/AIC_PatrolEnemyController` (`Pawn.GetController` _asbp_patrol_enemy) :!pure true) (`self.K2_GetActorLocation` (`GameplayStatics.GetPlayerPawn` 0)))))))
      (:`then_1`
        (`KismetSystemLibrary.RetriggerableDelay` 0.5)
        (`BlackboardComponent.ClearValue` (`self.Blackboard`) "TargetActor")
        (bind _outactors (`GameplayStatics.GetAllActorsOfClass` "/Game/GenericGame/Blueprints/Characters/BP_PatrolEnemy.BP_PatrolEnemy_C"))
        (for _array_element_2 _outactors
          (bind _asaic_patrol_enemy_controller (cast `/Game/GenericGame/Blueprints/AI/AIC_PatrolEnemyController` (`Pawn.GetController` _array_element_2)))
          (`/Game/GenericGame/Blueprints/AI/AIC_PatrolEnemyController.OnStopAlert` _asaic_patrol_enemy_controller))
        (goto _label :!via `Reset`)))))

(event `self.PawnSensing.OnHearNoise`
  (params (Instigator :type "Pawn Object Reference") (Location :type "Vector Structure (by ref)") (Volume :type "Float (single-precision)"))
  ;[1 1 1] documented
  (if (== (cast `Character` Instigator :!pure true) (`GameplayStatics.GetPlayerCharacter` 0))
    (`BlackboardComponent.SetValueAsVector` (`self.Blackboard`) "InvestigationLocation" Location)))

(fn `UserConstructionScript`)