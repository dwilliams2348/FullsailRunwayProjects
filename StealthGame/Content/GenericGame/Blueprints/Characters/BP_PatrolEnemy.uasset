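; Patrol enemy character that attacks the first-person player on contact and can be killed by a takedown.
; Overlapping PlayerHitZone calls the player's OnHit, then a timer restores CanAttack after AttackCooldown.
; OnTakedown messages its controller to stop the chase, disables capsule collision, removes the AI controller's detection meter, ragdolls the mesh and destroys the actor after a delay.
; The enemy's own OnHit event is empty.
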(event `self.ReceiveBeginPlay`)

(event `/Game/GenericGame/Blueprints/Interfaces/BPI_Combat.OnHit`
  (params (Damage :type "Float (double-precision)")))

(event `/Game/GenericGame/Blueprints/Interfaces/BPI_Combat.OnTakedown`
  (bind _returnvalue (`self.GetController`))
  (bind _asaic_patrol_enemy_controller (cast `/Game/GenericGame/Blueprints/AI/AIC_PatrolEnemyController` _returnvalue :!pure true))
  ;[1 1 1] documented
  (message `/Game/GenericGame/Blueprints/Interfaces/BPI_Detection.StopChase` _returnvalue)
  (`PrimitiveComponent.SetCollisionEnabled` (`self.CapsuleComponent`) "NoCollision")
  (`Widget.RemoveFromParent` (`/Game/GenericGame/Blueprints/AI/AIC_PatrolEnemyController.DetectionMeter` _asaic_patrol_enemy_controller))
  (set `/Game/GenericGame/Blueprints/AI/AIC_PatrolEnemyController.bShouldRotateMeter` false _asaic_patrol_enemy_controller)
  (`self.DeathRagdoll`)
  (`KismetSystemLibrary.Delay` 2.0)
  (`self.K2_DestroyActor`))

(event `DeathRagdoll`
  ;[1 1 1] documented
  (`SkeletalMeshComponent.SetAllBodiesSimulatePhysics` (`self.Mesh`) true))

(event `self.PlayerHitZone.OnComponentBeginOverlap`
  (params (OverlappedComponent :type "PrimitiveComponent Object Reference") (OtherActor :type "Actor Object Reference") (OtherComp :type "PrimitiveComponent Object Reference") (OtherBodyIndex :type Integer) (bFromSweep :type Boolean) (SweepResult :type "HitResult Structure (by ref)"))
  (bind _asbp_first_person_character (cast `/Game/GenericGame/Blueprints/Characters/BP_FirstPersonCharacter` OtherActor))
  (if (`self.bCanAttack`)
    (`/Game/GenericGame/Blueprints/Interfaces/BPI_Combat.OnHit` _asbp_first_person_character 0.0)
    (set `self.bCanAttack` false)
    (`KismetSystemLibrary.K2_SetTimerDelegate` (delegate `ResetAttack`) (`self.AttackCooldown`))))

(event `ResetAttack`
  (set `self.bCanAttack` true))

(fn `UserConstructionScript`)