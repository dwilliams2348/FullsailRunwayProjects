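; Base enemy character for a top-down game, handling health, AI startup and death.
; On BeginPlay it scales health by a multiplier and runs an assigned behavior tree with the player pawn as TargetActor.
; OnHit subtracts damage and triggers OnDeath at zero, which awards score to the player, stops AI logic, ragdolls the mesh and destroys the actor after a delay.
; The construction script applies MovementSpeed to walk speed.
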(event `self.ReceiveBeginPlay`
  ;[1 1 1] documented
  (set `self.CurrentHealth` (* (`self.BaseHealth`) (`self.HealthMult`)))
  (bind _asaicontroller (cast `AIController` (`self.GetController`)))
  (bind _behaviortreetorun (`self.BehaviorTreeToRun`)
    (:`then`
      (`AIController.RunBehaviorTree` _asaicontroller _behaviortreetorun)
      (`BlackboardComponent.SetValueAsObject` (`AIController.Blackboard` _asaicontroller) "TargetActor" (`GameplayStatics.GetPlayerPawn` 0)))
    (:`else`)))

(event `/Game/GenericGame/Blueprints/Interfaces/BPI_Combat.OnHit`
  (params (Damage :type "Float (double-precision)"))
  ;[1 1 1] documented
  (bind _output_get (set `self.CurrentHealth` (`KismetMathLibrary.FMax` (- (`self.CurrentHealth`) Damage))))
  (if (not (> _output_get 0.0))
    (`PrimitiveComponent.SetCollisionResponseToChannel` (`self.CapsuleComponent`) "ECC_GameTraceChannel1" "ECR_Ignore")
    (`self.OnDeath`)))

(event `OnDeath`
  ;[1 1 1] documented
  (bind _asbp_top_down_character (cast `/Game/GenericGame/Blueprints/Characters/BP_TopDownCharacter` (`GameplayStatics.GetPlayerCharacter` 0)))
  (`/Game/GenericGame/Blueprints/Characters/BP_TopDownCharacter.UpdatePlayerScore` _asbp_top_down_character (`self.ScoreValue`))
  (`BrainComponent.StopLogic` (`AIController.BrainComponent` (`AIBlueprintHelperLibrary.GetAIController` self)) "Dead")
  (`PrimitiveComponent.SetCollisionEnabled` (`self.CapsuleComponent`) "NoCollision")
  (`SkeletalMeshComponent.SetAllBodiesSimulatePhysics` (`self.Mesh`) true)
  (`KismetSystemLibrary.Delay` 2.5)
  (`self.K2_DestroyActor`))

(fn `UserConstructionScript`
  (set `CharacterMovementComponent.MaxWalkSpeed` (`self.MovementSpeed`) (`self.CharacterMovement`)))