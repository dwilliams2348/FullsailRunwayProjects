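; BP_ProjectileEnemy is an AI-controlled enemy character Blueprint that feeds state to its Blackboard.
; On BeginPlay it writes MovementSwitchInterval to the MovementTypeSwitch key.
; AsyncEvent starts a one-shot timer of that same interval, unless one is already valid.
; When the timer fires, ResetBlackboardKey clears the TargetActor key and invalidates the handle so the timer can be started again.
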(event `self.ReceiveBeginPlay`
  ;[1 1 1] documented
  (`parent.ReceiveBeginPlay`)
  (bind _asaicontroller (cast `AIController` (`self.GetController`)))
  (`BlackboardComponent.SetValueAsFloat` (`AIController.Blackboard` _asaicontroller) "MovementTypeSwitch" (`self.MovementSwitchInterval`)))

(event `AsyncEvent`
  ;[1 1 1] documented
  (if (not (`KismetSystemLibrary.K2_IsValidTimerHandle` (`self.TimerHandle`)))
    (bind _returnvalue (`KismetSystemLibrary.K2_SetTimerDelegate` (delegate `ResetBlackboardKey`) (`self.MovementSwitchInterval`)))
    (set `self.TimerHandle` _returnvalue)))

(event `ResetBlackboardKey`
  ;[1 1 1] documented
  (bind _asaicontroller (cast `AIController` (`self.GetController`)))
  (`BlackboardComponent.ClearValue` (`AIController.Blackboard` _asaicontroller) "TargetActor")
  (`KismetSystemLibrary.K2_ClearAndInvalidateTimerHandle` (`self.TimerHandle`)))

(fn `UserConstructionScript`
  (`parent.UserConstructionScript`))