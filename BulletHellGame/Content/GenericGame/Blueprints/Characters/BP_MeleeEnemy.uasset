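; BP_MeleeEnemy is an enemy character that damages the player through contact with its melee zone.
; When a pawn entering MeleeZone is player 0's pawn, it sends that pawn an OnHitMessage carrying MeleeDamage, once per overlap begin.
; On death it destroys MeleeZone to stop further hits, then defers to the parent's OnDeath handling.
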(event `self.MeleeZone.OnComponentBeginOverlap`
  (params (OverlappedComponent :type "PrimitiveComponent Object Reference") (OtherActor :type "Actor Object Reference") (OtherComp :type "PrimitiveComponent Object Reference") (OtherBodyIndex :type Integer) (bFromSweep :type Boolean) (SweepResult :type "HitResult Structure (by ref)"))
  (bind _returnvalue (`GameplayStatics.GetPlayerPawn` 0))
  ;[1 1 1] documented
  (if (== (cast `Pawn` OtherActor :!pure true) _returnvalue)
    (message `/Game/GenericGame/Blueprints/Interfaces/BPI_Combat.OnHit` _returnvalue (`self.MeleeDamage`))))

(event `self.OnDeath`
  ;[1 1 1] documented
  (`ActorComponent.K2_DestroyComponent` (`self.MeleeZone`))
  (`parent.OnDeath`))

(fn `UserConstructionScript`
  (`parent.UserConstructionScript`))