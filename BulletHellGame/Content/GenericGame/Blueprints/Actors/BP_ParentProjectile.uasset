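; BP_ParentProjectile is a base projectile actor that damages characters it overlaps.
; Construction passes its Velocity variable to the ProjectileMovement component.
; On sphere overlap, ShouldHit accepts only characters other than the owner whose capsule response to GameTraceChannel1 differs from the owner's, using collision settings as an allegiance filter.
; A valid hit sends OnHitMessage with Damage to the target, then destroys the projectile.
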(event `self.ReceiveBeginPlay`)

(event `self.Sphere.OnComponentBeginOverlap`
  (params (OverlappedComponent :type "PrimitiveComponent Object Reference") (OtherActor :type "Actor Object Reference") (OtherComp :type "PrimitiveComponent Object Reference") (OtherBodyIndex :type Integer) (bFromSweep :type Boolean) (SweepResult :type "HitResult Structure (by ref)"))
  (bind _return (`self.ShouldHit` OtherActor))
  (if _return
    (message `/Game/GenericGame/Blueprints/Interfaces/BPI_Combat.OnHit` OtherActor (`self.Damage`))
    (`self.K2_DestroyActor`)))

(fn `ShouldHit`
  (params (HitActor :type "Actor Object Reference"))
  (returns (Return :type Boolean))
  (bind _owningcharacter (`self.OwningCharacter`))
  (bind _ascharacter (cast `Character` HitActor))
  (if (== _ascharacter _owningcharacter)
    (return false)
    (else
      (return (not (`|EnumEquality` (`PrimitiveComponent.GetCollisionResponseToChannel` (`Character.CapsuleComponent` _owningcharacter) "ECC_GameTraceChannel1") (`PrimitiveComponent.GetCollisionResponseToChannel` (`Character.CapsuleComponent` _ascharacter) "ECC_GameTraceChannel1")))))))

(fn `UserConstructionScript`
  ;[1 1 1] Documented
  (set `MovementComponent.Velocity` (`self.Velocity`) (`self.ProjectileMovement`)))